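; Traffic spawner actor that keeps spawning random buses, cars and trucks at its own location.
; Tick runs through a random Delay, acting as a repeating timer that calls the Spawner function.
; Spawner randomly picks a vehicle type, then one of three color variants.
; Each spawn resets the delay range by type, so cars leave the shortest gap before the next vehicle and trucks the longest.
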(event EventBeginPlay)

(event Collision|EventActorBeginOverlap
  (params (OtherActor :type Actor%20Object%20Reference)))

(event EventTick
  (params (DeltaSeconds :type Float%20%28single-precision%29))
  (Utilities|FlowControl|Delay (Math|Random|RandomFloatinRange (Variables|Default|GetDelayMin) (Variables|Default|GetDelayMax)))
  (CallFunction|Spawner (Transformation|GetActorLocation)))

(fn ConstructionScript)

(fn Spawner
  (params (Location :type Vector))
  (switch int (Math|Random|RandomIntegerinRange 0 2)
    (:0
      (switch int (Math|Random|RandomIntegerinRange 0 2)
        (:0
          (Game|SpawnActorfromClass "/Game/Blueprints/BP_Bus_Purple_Child.BP_Bus_Purple_Child_C" (Math|Transform|MakeTransform Location "0, 0, 0" "1,1,1") "Undefined" 0 0)
          (Variables|Default|SetDelayMin 4.0)
          (Variables|Default|SetDelayMax 5.0))
        (:1
          (Game|SpawnActorfromClass "/Game/Blueprints/BP_Bus_Yellow_Child.BP_Bus_Yellow_Child_C" (Math|Transform|MakeTransform Location "0, 0, 0" "1,1,1") "Undefined" 0 0)
          (Variables|Default|SetDelayMin 4.0)
          (Variables|Default|SetDelayMax 5.0))
        (:2
          (Game|SpawnActorfromClass "/Game/Blueprints/BP_Bus_Red.BP_Bus_Red_C" (Math|Transform|MakeTransform Location "0, 0, 0" "1,1,1") "Undefined" 0 0)
          (Variables|Default|SetDelayMin 4.0)
          (Variables|Default|SetDelayMax 5.0))))
    (:1
      (switch int (Math|Random|RandomIntegerinRange 0 2)
        (:0
          (Game|SpawnActorfromClass "/Game/Blueprints/BP_Car_Red.BP_Car_Red_C" (Math|Transform|MakeTransform Location "0, 0, 0" "1,1,1") "Undefined" 0 0)
          (Variables|Default|SetDelayMin 2.0)
          (Variables|Default|SetDelayMax 3.0))
        (:1
          (Game|SpawnActorfromClass "/Game/Blueprints/BP_Car_Blue_Child.BP_Car_Blue_Child_C" (Math|Transform|MakeTransform Location "0, 0, 0" "1,1,1") "Undefined" 0 0)
          (Variables|Default|SetDelayMin 2.0)
          (Variables|Default|SetDelayMax 3.0))
        (:2
          (Game|SpawnActorfromClass "/Game/Blueprints/BP_Car_Green_Child.BP_Car_Green_Child_C" (Math|Transform|MakeTransform Location "0, 0, 0" "1,1,1") "Undefined" 0 0)
          (Variables|Default|SetDelayMin 2.0)
          (Variables|Default|SetDelayMax 3.0))))
    (:2
      (switch int (Math|Random|RandomIntegerinRange 0 2)
        (:0
          (Game|SpawnActorfromClass "/Game/Blueprints/BP_Truck_Red.BP_Truck_Red_C" (Math|Transform|MakeTransform Location "0, 0, 0" "1,1,1") "Undefined" 0 0)
          (Variables|Default|SetDelayMin 1e+01)
          (Variables|Default|SetDelayMax 3e+01))
        (:1
          (Game|SpawnActorfromClass "/Game/Blueprints/BP_Truck_Blue_Child.BP_Truck_Blue_Child_C" (Math|Transform|MakeTransform Location "0, 0, 0" "1,1,1") "Undefined" 0 0)
          (Variables|Default|SetDelayMin 1e+01)
          (Variables|Default|SetDelayMax 3e+01))
        (:2
          (Game|SpawnActorfromClass "/Game/Blueprints/BP_Truck_Pink_Child.BP_Truck_Pink_Child_C" (Math|Transform|MakeTransform Location "0, 0, 0" "1,1,1") "Undefined" 0 0)
          (Variables|Default|SetDelayMin 1e+01)
          (Variables|Default|SetDelayMax 3e+01))))))