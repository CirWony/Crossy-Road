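; Player Blueprint for hop-based movement: each MoveForward or MoveRight release triggers a short jump, turns the mesh and offsets the actor with sweep by axis value times Speed.
; An IsJumping flag blocks new hops until the current one ends, then the Eagle timeline restarts as an idle countdown.
; When that timeline finishes, an eagle sound plays and GM_Tutorial restarts the game, as it does when Tick detects a fast fall.
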(event EventTick
  (params (DeltaSeconds :type Float%20%28single-precision%29))
  (if (< (.Z (Math|Vector|BreakVector (Transformation|GetVelocity))) -2e+03)
    (bind _asgm_tutorial (Utilities|Casting|CastToGM_Tutorial (Game|GetGameMode)))
    (Class|GameMode|RestartGame _asgm_tutorial)))

(event Input|ActionEvents|InputActionMoveForward
  (params (Key :type Key%20Structure))
  (bind _mesh (Variables|Character|GetMesh))
  (:Released
    (if (not (Variables|Default|GetisJumping))
      (Character|Jump)
      (Variables|Default|SetisJumping true)
      (if (> (stale Input|AxisEvents|InputAxisMoveForward AxisValue) 0.0)
        (Transformation|SetRelativeRotation _mesh "0,270.000000, 0" false false)
        (else
          (Transformation|SetRelativeRotation _mesh "0,90.000000, 0" false false)))
      (Transformation|AddActorLocalOffset (* (Transformation|GetActorForwardVector) (* (stale Input|AxisEvents|InputAxisMoveForward AxisValue) (Variables|Default|GetSpeed))) true false)
      (Utilities|FlowControl|Delay 0.4)
      (Character|StopJumping)
      (Variables|Default|SetisJumping false)
      (Timeline|Eagle PlayFromStart
        (:Finished
          (Audio|PlaySoundatLocation "/Game/Audio/eagle.eagle" (Transformation|GetActorLocation) "0, 0, 0" 1.0 1.0 0.0 0 0 0)
          (Utilities|FlowControl|Delay 2.0)
          (bind _asgm_tutorial (Utilities|Casting|CastToGM_Tutorial (Game|GetGameMode)))
          (Class|GameMode|RestartGame _asgm_tutorial))))))

(event Input|ActionEvents|InputActionMoveRight
  (params (Key :type Key%20Structure))
  (bind _mesh (Variables|Character|GetMesh))
  (:Released
    (if (not (Variables|Default|GetisJumping))
      (Character|Jump)
      (Variables|Default|SetisJumping true)
      (if (> (stale Input|AxisEvents|InputAxisMoveRight AxisValue) 0.0)
        (Transformation|SetRelativeRotation _mesh "0, 0, 0" false false)
        (else
          (Transformation|SetRelativeRotation _mesh "0,180.000000, 0" false false)))
      (Transformation|AddActorLocalOffset (* (Transformation|GetActorRightVector) (* (stale Input|AxisEvents|InputAxisMoveRight AxisValue) (Variables|Default|GetSpeed))) true false)
      (Utilities|FlowControl|Delay 0.4)
      (Character|StopJumping)
      (Variables|Default|SetisJumping false)
      (Timeline|Eagle PlayFromStart
        (:Finished
          (Audio|PlaySoundatLocation "/Game/Audio/eagle.eagle" (Transformation|GetActorLocation) "0, 0, 0" 1.0 1.0 0.0 0 0 0)
          (Utilities|FlowControl|Delay 2.0)
          (bind _asgm_tutorial (Utilities|Casting|CastToGM_Tutorial (Game|GetGameMode)))
          (Class|GameMode|RestartGame _asgm_tutorial))))))

(event Input|AxisEvents|InputAxisMoveForward
  (params (AxisValue :type Float%20%28single-precision%29)))

(event Input|AxisEvents|InputAxisMoveRight
  (params (AxisValue :type Float%20%28single-precision%29)))

(fn ConstructionScript)