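; Game mode for a lane-crossing game that builds a random tile course and tracks jump and coin scores.
; BeginPlay calls SpawnTile 16 times, each picking grass, road, water, train track or lily-pad water at random.
; Each new tile spawns its own props, hazards or coins, then its SpawnPoint location becomes the next spawn transform, chaining tiles end to end.
; Two events add to JumpScore and to Score for coins.
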(event Custom|AddCoinScore
  (params (Add :type Integer))
  (Variables|Default|SetScore (+ Add (Variables|Default|GetScore))))

(event Custom|AddJumpScore
  (params (Add :type Integer))
  (Variables|Default|SetJumpScore (+ Add (Variables|Default|GetJumpScore))))

(event EventBeginPlay
  (for _index (range 0 15)
    (CallFunction|SpawnTile)))

(fn ConstructionScript)

(fn SpawnTile
  (switch int (Math|Random|RandomIntegerinRange 0 4)
    (:0
      (bind _returnvalue (Game|SpawnActorfromClass "/Game/Procedural/MasterTile_Grass.MasterTile_Grass_C" (Variables|Default|GetNextSpawnPoint) "Undefined" 0 0))
      (bind _asmaster_tile_grass (Utilities|Casting|CastToMasterTile_Grass _returnvalue))
      (Default|SpawnShrubbery _asmaster_tile_grass)
      (Variables|Default|SetNextSpawnPoint (Math|Transform|MakeTransform (Transformation|GetWorldLocation (Variables|/Game/Procedural/MasterTile_Grass.MasterTile_Grass_C|GetSpawnPoint _asmaster_tile_grass)) "0, 0, 0" "1,1,1")))
    (:1
      (bind _returnvalue_2 (Game|SpawnActorfromClass "/Game/Procedural/MasterTile_Road.MasterTile_Road_C" (Variables|Default|GetNextSpawnPoint) "Undefined" 0 0))
      (bind _asmaster_tile_road (Utilities|Casting|CastToMasterTile_Road _returnvalue_2))
      (Default|SpawnCars _asmaster_tile_road)
      (Default|SpawnCoins _asmaster_tile_road)
      (Variables|Default|SetNextSpawnPoint (Math|Transform|MakeTransform (Transformation|GetWorldLocation (Variables|/Game/Procedural/MasterTile_Road.MasterTile_Road_C|GetSpawnPoint _asmaster_tile_road)) "0, 0, 0" "1,1,1")))
    (:2
      (bind _returnvalue_3 (Game|SpawnActorfromClass "/Game/Procedural/MasterTile_Water.MasterTile_Water_C" (Variables|Default|GetNextSpawnPoint) "Undefined" 0 0))
      (bind _asmaster_tile_water (Utilities|Casting|CastToMasterTile_Water _returnvalue_3))
      (Default|SpawnLogs _asmaster_tile_water)
      (Variables|Default|SetNextSpawnPoint (Math|Transform|MakeTransform (Transformation|GetWorldLocation (Variables|/Game/Procedural/MasterTile_Water.MasterTile_Water_C|GetSpawnPoint _asmaster_tile_water)) "0, 0, 0" "1,1,1")))
    (:3
      (bind _returnvalue_4 (Game|SpawnActorfromClass "/Game/Procedural/MasterTile_Track.MasterTile_Track_C" (Variables|Default|GetNextSpawnPoint) "Undefined" 0 0))
      (bind _asmaster_tile_track (Utilities|Casting|CastToMasterTile_Track _returnvalue_4))
      (Default|SpawnTrain _asmaster_tile_track)
      (Variables|Default|SetNextSpawnPoint (Math|Transform|MakeTransform (Transformation|GetWorldLocation (Variables|/Game/Procedural/MasterTile_Track.MasterTile_Track_C|GetSpawnPoint _asmaster_tile_track)) "0, 0, 0" "1,1,1")))
    (:4
      (bind _returnvalue_5 (Game|SpawnActorfromClass "/Game/Procedural/MasterTile_WaterPad.MasterTile_WaterPad_C" (Variables|Default|GetNextSpawnPoint) "Undefined" 0 0))
      (bind _asmaster_tile_water_pad (Utilities|Casting|CastToMasterTile_WaterPad _returnvalue_5))
      (Default|SpawnLilyPads _asmaster_tile_water_pad)
      (Variables|Default|SetNextSpawnPoint (Math|Transform|MakeTransform (Transformation|GetWorldLocation (Variables|/Game/Procedural/MasterTile_WaterPad.MasterTile_WaterPad_C|GetSpawnPoint _asmaster_tile_water_pad)) "0, 0, 0" "1,1,1")))))