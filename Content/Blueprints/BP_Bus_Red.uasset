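; BP_Bus_Red is a red bus hazard that drives continuously and kills the player on impact.
; Each Tick it offsets itself by its right vector times MaxSpeed, without sweep or delta-time scaling.
; A StaticMesh hit on BP_Player squashes the player's mesh by rescaling it and spawns the PS_Hit emitter at the bus.
; After a short delay, it calls RestartGame on GM_Tutorial.
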(event OnComponentHit(StaticMesh)
  (params (HitComponent :type Primitive%20Component%20Object%20Reference) (OtherActor :type Actor%20Object%20Reference) (OtherComp :type Primitive%20Component%20Object%20Reference) (NormalImpulse :type Vector :default "0, 0, 0") (Hit :type Hit%20Result%20Structure%20%28by%20ref%29))
  (bind _asbp_player (Utilities|Casting|CastToBP_Player OtherActor))
  (Transformation|SetWorldScale3D (Variables|/Script/Engine.Character|GetMesh _asbp_player) "0.100000,0.010000,0.100000")
  (Effects|SpawnEmitteratLocation "/Game/Particles/PS_Hit.PS_Hit" (Transformation|GetActorLocation))
  (Utilities|FlowControl|Delay 0.5)
  (bind _asgm_tutorial (Utilities|Casting|CastToGM_Tutorial (Game|GetGameMode)))
  (Class|GameMode|RestartGame _asgm_tutorial))

(event EventBeginPlay)

(event Collision|EventActorBeginOverlap
  (params (OtherActor :type Actor%20Object%20Reference)))

(event EventTick
  (params (DeltaSeconds :type Float%20%28single-precision%29))
  (Transformation|AddActorLocalOffset (* (Transformation|GetActorRightVector) (Variables|Default|GetMaxSpeed)) false false))

(fn ConstructionScript)