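; BP_Train_Spawner is an actor that repeatedly spawns trains at its own location at random intervals.
; On BeginPlay it finds the first BP_TrainPost, then loops: random delay, flag the post as incoming, spawn a BP_Train five seconds later, and clear the flag shortly after.
; The Spawner function also resets the random delay range after each spawn, so the starting range applies only to the first train.
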(event EventBeginPlay
  (bind _outactors (Actor|GetAllActorsOfClass "/Game/Blueprints/BP_TrainPost.BP_TrainPost_C"))
  (Variables|Default|SetTrainPostLight (Utilities|Array|Get(acopy) _outactors))
  (Utilities|FlowControl|Delay (Math|Random|RandomFloatinRange (Variables|Default|GetDelayMin) (Variables|Default|GetDelayMax)) :!label _label)
  (bind _asbp_train_post (Utilities|Casting|CastToBP_TrainPost (Variables|Default|GetTrainPostLight)))
  (Variables|/Game/Blueprints/BP_TrainPost.BP_TrainPost_C|SetisIncoming _asbp_train_post true)
  (Utilities|FlowControl|Delay 5.0)
  (CallFunction|Spawner (Transformation|GetActorLocation))
  (Utilities|FlowControl|Delay 2.0)
  (bind _asbp_train_post_2 (Utilities|Casting|CastToBP_TrainPost (Variables|Default|GetTrainPostLight)))
  (Variables|/Game/Blueprints/BP_TrainPost.BP_TrainPost_C|SetisIncoming _asbp_train_post_2 false)
  (goto _label))

(event EventTick
  (params (DeltaSeconds :type Float%20%28single-precision%29)))

(fn ConstructionScript)

(fn Spawner
  (params (Location :type Vector))
  (Game|SpawnActorfromClass "/Game/Blueprints/BP_Train.BP_Train_C" (Math|Transform|MakeTransform Location "0, 0, 0" "1,1,1") "Undefined" 0 0)
  (Variables|Default|SetDelayMin 1e+01)
  (Variables|Default|SetDelayMax 25.0))